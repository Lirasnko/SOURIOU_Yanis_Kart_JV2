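; BP_AC_LapCheck is a lap-tracking component that counts laps for its owner in a vehicle game.
; AddLap compares the number of entries in its Checkpoints list with the AllCheckpoint list on BP_VehicleAdvGameMode.
; When the counts match, it increments Lap and clears Checkpoints for the next lap.
; The check is by count only, and nothing in its graphs fills Checkpoints or calls AddLap.
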(event EventBeginPlay)

(event EventTick
  (params (DeltaSeconds :type Float%20%28single-precision%29)))

(fn AddLap
  (bind _asbp_vehicle_adv_game_mode (Utilities|Casting|CastToBP_VehicleAdvGameMode (Game|GetGameMode)))
  (if (== (Utilities|Array|Length (Variables|/Game/VehicleTemplate/Blueprints/BP_VehicleAdvGameMode.BP_VehicleAdvGameMode_C|GetAllCheckpoint _asbp_vehicle_adv_game_mode)) (Utilities|Array|Length (Variables|Default|GetCheckpoints)))
    (bind _result (Math|Integer|IncrementInt (Variables|Default|GetLap))
      (:%20%20
        (Variables|Default|SetLap _result)
        (Utilities|Array|Clear (Variables|Default|GetCheckpoints))))))