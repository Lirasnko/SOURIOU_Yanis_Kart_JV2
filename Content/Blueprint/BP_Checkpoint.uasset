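; BP_Checkpoint is a race track checkpoint that records which vehicles pass through it.
; On BeginPlay it registers itself in the vehicle game mode's AllCheckpoint list.
; When a vehicle pawn enters its box, it adds itself uniquely to the Checkpoints array on that controller's BP_AC_LapCheck component, then prints every collected checkpoint name as debug output.
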(event OnComponentBeginOverlap(Box)
  (params (OverlappedComponent :type Primitive%20Component%20Object%20Reference) (OtherActor :type Actor%20Object%20Reference) (OtherComp :type Primitive%20Component%20Object%20Reference) (OtherBodyIndex :type Integer) (bFromSweep :type Boolean) (SweepResult :type Hit%20Result%20Structure%20%28by%20ref%29))
  (bind _asbp_vehicle_adv_pawn_base (Utilities|Casting|CastToBP_VehicleAdvPawnBase OtherActor))
  (Utilities|IsValid (Actor|GetComponentbyClass (Pawn|GetController _asbp_vehicle_adv_pawn_base) "/Game/Blueprint/BP_AC_LapCheck.BP_AC_LapCheck_C")
    (:Is%20Valid
      (Utilities|Array|AddUnique (Variables|/Game/Blueprint/BP_AC_LapCheck.BP_AC_LapCheck_C|GetCheckpoints (Actor|GetComponentbyClass (Pawn|GetController _asbp_vehicle_adv_pawn_base) "/Game/Blueprint/BP_AC_LapCheck.BP_AC_LapCheck_C")) self)
      (for _array_element (Variables|/Game/Blueprint/BP_AC_LapCheck.BP_AC_LapCheck_C|GetCheckpoints (Actor|GetComponentbyClass (Pawn|GetController _asbp_vehicle_adv_pawn_base) "/Game/Blueprint/BP_AC_LapCheck.BP_AC_LapCheck_C"))
        (Development|PrintString (Utilities|GetDisplayName _array_element))))))

(event EventBeginPlay
  (bind _asbp_vehicle_adv_game_mode (Utilities|Casting|CastToBP_VehicleAdvGameMode (Game|GetGameMode)))
  (Utilities|Array|AddUnique (Variables|/Game/VehicleTemplate/Blueprints/BP_VehicleAdvGameMode.BP_VehicleAdvGameMode_C|GetAllCheckpoint _asbp_vehicle_adv_game_mode) self))

(event Collision|EventActorBeginOverlap
  (params (OtherActor :type Actor%20Object%20Reference)))

(event EventTick
  (params (DeltaSeconds :type Float%20%28single-precision%29)))

(fn ConstructionScript)