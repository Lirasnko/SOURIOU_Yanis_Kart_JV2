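; BP_GreenShell is a projectile that travels at a set speed, damages vehicles and bounces off other obstacles.
; Tick moves it along its velocity without sweeping and spins its sphere.
; Capsule overlap with a vehicle pawn calls TakeDamage on its player controller and destroys the shell.
; Other overlaps trace forward, with persistent debug drawing, and reflect heading off the hit normal, destroying the shell once the bounce limit is reached.
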(event OnComponentBeginOverlap(Capsule)
  (params (OverlappedComponent :type Primitive%20Component%20Object%20Reference) (OtherActor :type Actor%20Object%20Reference) (OtherComp :type Primitive%20Component%20Object%20Reference) (OtherBodyIndex :type Integer) (bFromSweep :type Boolean) (SweepResult :type Hit%20Result%20Structure%20%28by%20ref%29))
  (bind _returnvalue (Transformation|GetActorLocation))
  (bind _capsule (Variables|Default|GetCapsule))
  (bind _bounce (Variables|Default|GetBounce))
  (bind _returnvalue_2 (Math|Vector|GetForwardVector _capsule))
  (bind _returnvalue_3 (* _returnvalue_2 75))
  (bind _asbp_vehicle_adv_pawn_base (Utilities|Casting|CastToBP_VehicleAdvPawnBase OtherActor)
    (:then
      (bind _asbp_vehicle_adv_player_controller (Utilities|Casting|CastToBP_VehicleAdvPlayerController (Pawn|GetController _asbp_vehicle_adv_pawn_base)))
      (Default|TakeDamage _asbp_vehicle_adv_player_controller)
      (Actor|DestroyActor :!label _label))
    (:CastFailed
      (if (!= _bounce (Variables|Default|GetMaxBounce))
        (Math|Integer|IncrementInt _bounce
          (:%20%20
            (bind _outhit (Collision|LineTraceByChannel _returnvalue (+ _returnvalue _returnvalue_3) "TraceTypeQuery1" false 0 "Persistent"))
            (Transformation|SetRelativeRotation (Variables|Default|GetCapsule) (Math|Rotator|MakeRotfromX (Math|Vector|GetReflectionVector _returnvalue_3 (.normal _outhit))) false false)
            (Variables|Default|SetVelocity (* (Math|Vector|GetForwardVector (Variables|Default|GetCapsule)) (Variables|Default|GetSpeed)))))
        (else
          (goto _label))))))

(event EventBeginPlay
  (Variables|Default|SetVelocity (* (Math|Vector|GetForwardVector (Variables|Default|GetCapsule)) (Variables|Default|GetSpeed))))

(event EventTick
  (params (DeltaSeconds :type Float%20%28single-precision%29))
  (bind _sphere (Variables|Default|GetSphere))
  (Transformation|SetActorLocation (+ (Transformation|GetActorLocation) (* (Variables|Default|GetVelocity) DeltaSeconds)) false false)
  (Transformation|SetRelativeRotation _sphere (Math|Rotator|CombineRotators (Variables|/Script/Engine.SceneComponent|GetRelativeRotation _sphere) "0.000000,5.000000,0.000000") false false))

(fn ConstructionScript)